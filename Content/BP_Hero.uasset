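; BP_Hero is the third-person player character, handling Enhanced Input movement, look with optional axis inversion, jump, roll and slide.
; A timeline ramps walk speed when movement starts, scaling jump velocity and, in Tick, camera arm length with it.
; Timelines nudge the actor forward without sweep for airborne jumps, run-to-stop, rolls and slides.
; ABP_Hero flags signal stop, roll and slide, with delays gating repeats and a timeline restoring the camera after stopping.
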(event `self.ReceiveBeginPlay`
  (bind _charactermovement (`self.CharacterMovement`))
  (bind _returnvalue (pcsubsystem `EnhancedInputLocalPlayerSubsystem` (`GameplayStatics.GetPlayerController` 0)))
  (bind _jumpzvelocity (`CharacterMovementComponent.JumpZVelocity` _charactermovement))
  ;[0.15 0.15 0.15 0.5 34] Void Start
  (`/Engine/EditorBlueprintResources/StandardMacros.IsValid` _returnvalue
    (:`Is Valid`
      (`EnhancedInputSubsystemInterface.AddMappingContext` _returnvalue "/Game/IMC_ThirdPerson.IMC_ThirdPerson" 0 (struct))
      (set `self.BaseSpeed` (`MovementComponent.GetMaxSpeed` _charactermovement))
      (set `self.BaseJumpHeight` _jumpzvelocity)
      (`KismetSystemLibrary.PrintText` (`KismetTextLibrary.Conv_DoubleToText` _jumpzvelocity "HalfToEven"))
      (set `self.AnimInstance` (`SkeletalMeshComponent.GetAnimInstance` (`self.Mesh`)))
      (set `self.BaseCamArmLength` (`SpringArmComponent.TargetArmLength` (`self.SelfieStick`))))))

(event `EnhancedInput|/Game/INP_Jump`
  (params (ActionValue :type Boolean) (ElapsedSeconds :type "Float (double-precision)") (TriggeredSeconds :type "Float (double-precision)") (InputAction :type "InputAction Object Reference" :default "/Game/INP_Jump.INP_Jump"))
  (bind _returnvalue (`self.K2_GetActorLocation`))
  (bind _charactermovement (`self.CharacterMovement`))
  ;[0.15 0.15 0.15 0.5 34] Jumping Handler
  (:`Started`
    (if (not (`NavMovementComponent.IsFalling` (`self.CharacterMovement`)))
      (`self.Jump`)
      (bind (_direction _jumpforwardtrack) (`Timeline|JumpTimeline` :!via `PlayFromStart`)
        (:`Update`
          (if (`NavMovementComponent.IsFalling` _charactermovement)
            (`self.K2_SetActorLocation` (`KismetMathLibrary.VLerp` _returnvalue (+ _returnvalue (* (`self.GetActorForwardVector`) (/ (`CharacterMovementComponent.MaxWalkSpeed` _charactermovement) 100.0))) _jumpforwardtrack)))))))
  (:`Completed`
    (`self.StopJumping`)))

(event `EnhancedInput|/Game/INP_MoveAround`
  (params (ActionValue :type "Vector2D Structure") (ElapsedSeconds :type "Float (double-precision)") (TriggeredSeconds :type "Float (double-precision)") (InputAction :type "InputAction Object Reference" :default "/Game/INP_MoveAround.INP_MoveAround"))
  (bind _returnvalue (`self.K2_GetActorLocation`))
  (bind (_returnvalue_roll _returnvalue_pitch _returnvalue_yaw) (`KismetMathLibrary.BreakRotator` (`self.GetControlRotation`)))
  (bind _charactermovement (`self.CharacterMovement`))
  (bind _selfiestick (`self.SelfieStick`))
  ;[0.15 0.15 0.15 0.5 34] Movement Handler
  (:`Triggered`
    (`self.AddMovementInput` (`KismetMathLibrary.GetRightVector` (`self.GetControlRotation`)) ActionValue_X)
    (`self.AddMovementInput` (`KismetMathLibrary.GetForwardVector` (`KismetMathLibrary.MakeRotator` _returnvalue_roll 0.0 _returnvalue_yaw)) ActionValue_Y))
  (:`Started`
    (bind (_direction _speed_ramp) (`Timeline|Ramp Up Speed` :!via `PlayFromStart`)
      (:`Update`
        (set `CharacterMovementComponent.MaxWalkSpeed` (* (.x _speed_ramp) (`self.BaseSpeed`)) _charactermovement)
        (set `CharacterMovementComponent.JumpZVelocity` (* (`self.BaseJumpHeight`) (/ (`CharacterMovementComponent.MaxWalkSpeed` _charactermovement) 600.0)) _charactermovement))))
  (:`Completed`
    (`KismetSystemLibrary.PrintString` "Released")
    (if (>= (`CharacterMovementComponent.MaxWalkSpeed` (`self.CharacterMovement`)) 850.0)
      (set `CharacterMovementComponent.MaxWalkSpeed` (`self.BaseSpeed`) _charactermovement)
      (set `self.CurrentLocation` _returnvalue)
      (bind (_direction_2 _runtostoptrack) (`Timeline|Run To Stop Timeline` :!via `PlayFromStart`)
        (:`Update`
          (`self.K2_SetActorLocation` (`KismetMathLibrary.VLerp` _returnvalue (+ _returnvalue (* (`self.GetActorForwardVector`) 6.0)) _runtostoptrack))
          (bind _asabp_hero (cast `/Game/ABP_Hero` (`self.AnimInstance`)))
          (set `/Game/ABP_Hero.IsStopping` true _asabp_hero))
        (:`Finished`
          (`KismetSystemLibrary.PrintText` "Hello")
          (`KismetSystemLibrary.Delay` 0.3)
          (set `/Game/ABP_Hero.IsStopping` false _asabp_hero)
          ;[0.15 0.15 0.15 0.5 34] Camera / LookAround Handler
          (bind (_direction_3 _revertcamtrack) (`Timeline|RevertCameraTimeline` :!via `PlayFromStart`)
            (:`Update`
              (set `SpringArmComponent.TargetArmLength` (`KismetMathLibrary.Lerp` (`SpringArmComponent.TargetArmLength` _selfiestick) (`self.BaseCamArmLength`) _revertcamtrack) _selfiestick))
            (:`Finished`)))))))

(event `self.ReceiveTick`
  (params (DeltaSeconds :type "Float (single-precision)"))
  (bind _charactermovement (`self.CharacterMovement`))
  ;[0.15 0.15 0.15 0.5 34] Camera / LookAround Handler
  (if (<= (+ (`self.BaseSpeed`) 10.0) (`MovementComponent.GetMaxSpeed` _charactermovement))
    (set `SpringArmComponent.TargetArmLength` (* (`self.BaseCamArmLength`) (/ (`CharacterMovementComponent.MaxWalkSpeed` _charactermovement) (`self.BaseSpeed`))) (`self.SelfieStick`))))

(event `EnhancedInput|/Game/INP_LookAround`
  (params (ActionValue :type "Vector2D Structure") (ElapsedSeconds :type "Float (double-precision)") (TriggeredSeconds :type "Float (double-precision)") (InputAction :type "InputAction Object Reference" :default "/Game/INP_LookAround.INP_LookAround"))
  ;[0.15 0.15 0.15 0.5 34] Camera / LookAround Handler
  (:`Triggered`
    (`self.AddControllerYawInput` (* ActionValue_X (`KismetMathLibrary.SelectFloat` -1.0 1.0 (`self.InvertCameraX`))))
    (`self.AddControllerPitchInput` (* (* ActionValue_Y (`KismetMathLibrary.SelectFloat` -1.0 1.0 (`self.InvertCameraY`))) 0.5))))

(event `EnhancedInput|/Game/INP_Roll`
  (params (ActionValue :type Boolean) (ElapsedSeconds :type "Float (double-precision)") (TriggeredSeconds :type "Float (double-precision)") (InputAction :type "InputAction Object Reference" :default "/Game/INP_Roll.INP_Roll"))
  (bind _returnvalue (`self.K2_GetActorLocation`))
  ;[0.15 0.15 0.15 0.5 34] Rolling Handler
  (:`Started`
    (if (not (`NavMovementComponent.IsFalling` (`self.CharacterMovement`)))
      (bind _asabp_hero (cast `/Game/ABP_Hero` (`self.AnimInstance`)))
      (if (not (`/Game/ABP_Hero.IsRolling` _asabp_hero))
        (if (`self.CanRoll`)
          (set `self.CanRoll` false)
          (bind _asabp_hero_2 (cast `/Game/ABP_Hero` (`self.AnimInstance`)))
          (set `/Game/ABP_Hero.IsRolling` true _asabp_hero_2)
          (bind (_direction _rolltrack) (`Timeline|RollTimeline` :!via `PlayFromStart`)
            (:`Update`
              (`self.K2_SetActorLocation` (`KismetMathLibrary.VLerp` _returnvalue (+ _returnvalue (* (`self.GetActorForwardVector`) 7.5)) _rolltrack))
              (`KismetSystemLibrary.Delay` 0.9466)
              (bind _asabp_hero_3 (cast `/Game/ABP_Hero` (`self.AnimInstance`)))
              (set `/Game/ABP_Hero.IsRolling` false _asabp_hero_3)
              (`KismetSystemLibrary.Delay` 0.25)
              (set `self.CanRoll` true))))))))

(event `EnhancedInput|/Game/INP_Slide`
  (params (ActionValue :type Boolean) (ElapsedSeconds :type "Float (double-precision)") (TriggeredSeconds :type "Float (double-precision)") (InputAction :type "InputAction Object Reference" :default "/Game/INP_Slide.INP_Slide"))
  (bind _returnvalue (`self.K2_GetActorLocation`))
  ;[0.15 0.15 0.15 0.5 34] Slide Handler
  (:`Started`
    (if (not (`NavMovementComponent.IsFalling` (`self.CharacterMovement`)))
      (bind _asabp_hero (cast `/Game/ABP_Hero` (`self.AnimInstance`)))
      (if (not (`/Game/ABP_Hero.IsSliding` _asabp_hero))
        (if (`self.CanSlide`)
          (set `self.CanSlide` false)
          (bind _asabp_hero_2 (cast `/Game/ABP_Hero` (`self.AnimInstance`)))
          (set `/Game/ABP_Hero.IsSliding` true _asabp_hero_2)
          (bind (_direction _rolltrack) (`Timeline|Timeline` :!via `PlayFromStart`)
            (:`Update`
              (`self.K2_SetActorLocation` (`KismetMathLibrary.VLerp` _returnvalue (+ _returnvalue (* (`self.GetActorForwardVector`) 7.5)) _rolltrack))
              (`KismetSystemLibrary.Delay` 0.9466)
              (bind _asabp_hero_3 (cast `/Game/ABP_Hero` (`self.AnimInstance`)))
              (set `/Game/ABP_Hero.IsSliding` false _asabp_hero_3)
              (`KismetSystemLibrary.Delay` 0.25)
              (set `self.CanSlide` true))))))))

(fn `UserConstructionScript`)